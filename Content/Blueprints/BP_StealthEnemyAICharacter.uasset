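; Stealth enemy AI character that draws its field of view as a flat vision cone mesh.
; On a looping timer, the authority runs the VisionCone EQS query and collects all matching locations as sight points.
; These become actor-relative vertices in a triangle fan, rebuilt as a procedural mesh with world rotation zeroed.
; SetConeMaterial swaps the material applied on each redraw.
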(event Custom|RunQuery
  (if (Ability|HasAuthority)
    (bind _returnvalue (AI|EQS|RunEQSQuery "/StealthEnemyAI/Blueprints/VisionCone.VisionCone" self "AllMatching"))
    (EventDispatchers|BindEventtoOnQueryFinishedEvent _returnvalue (delegate Custom|DrawVisionCone))))

(event Custom|DrawVisionCone
  (params (QueryInstance :type Env%20Query%20Instance%20Blueprint%20Wrapper%20Object%20Reference) (QueryStatus :type EEnvQueryStatus%20Enum :default "Processing"))
  (bind _resultlocations (AI|EQS|GetQueryResultsasLocations QueryInstance))
  (bind _output_get (Variables|Default|SetSightPoints _resultlocations))
  (bind (_vertices _triangles) (CallFunction|ConvertSightPointstoVertices _output_get))
  (CallFunction|DrawConeMesh _vertices _triangles))

(event Custom|DrawConeMesh
  (params (Vertices :type Array%20of%20Vectors) (Triangles :type Array%20of%20Integers))
  (bind _visioncone (Variables|Default|GetVisionCone))
  (Class|ProceduralMeshComponent|CreateMeshSectionLinearColor _visioncone 0 Vertices Triangles 0 0 0 0 0 0 0 false false)
  (Rendering|Material|SetMaterial _visioncone 0 (Variables|Default|GetConeMaterial))
  (Transformation|SetWorldRotation _visioncone "0, 0, 0" false false))

(event EventBeginPlay
  (|CallParentFunction)
  (Utilities|Array|Resize (Variables|Default|GetVertices) 51)
  (Utilities|Time|SetTimerbyEvent (delegate Custom|RunQuery) 0.3 true))

(event EventSetConeMaterial
  (params (MaterialInstance :type Material%20Instance%20Object%20Reference))
  (Variables|Default|SetConeMaterial MaterialInstance))

(fn ConstructionScript)

(fn ConvertSightPointstoVertices
  (params (SightPoints :type Array%20of%20Vectors))
  (bind _returnvalue (Transformation|GetActorLocation))
  (bind _vertices (Variables|Default|GetVertices))
  (bind _returnvalue_2 (Utilities|Array|Length _vertices))
  (bind (_x _y) (Math|Vector|BreakVector _returnvalue))
  (Utilities|Array|SetArrayElem :TargetArray (Variables|Default|GetVertices))
  (for (_array_element _array_index) SightPoints
    (Utilities|Array|SetArrayElem (Variables|Default|GetVertices) (+ _array_index 1) (Math|Vector|MakeVector (- (.X (Math|Vector|BreakVector _array_element)) _x) (- (.Y (Math|Vector|BreakVector _array_element)) _y) -5e+01)))
  (Utilities|Array|Resize (Variables|Default|GetTriangles) (* _returnvalue_2 3))
  (for _index (range 0 _returnvalue_2)
    (Utilities|Array|SetArrayElem (Variables|Default|GetTriangles) (* _index 3) 0)
    (Utilities|Array|SetArrayElem (Variables|Default|GetTriangles) (+ (* _index 3) 1) (+ _index 1))
    (Utilities|Array|SetArrayElem (Variables|Default|GetTriangles) (+ (+ (* _index 3) 1) 1) (+ (+ _index 1) 1)))
  (return (Variables|Default|GetVertices) (Variables|Default|GetTriangles)))